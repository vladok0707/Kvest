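; BP_ATM is an ATM actor with a Cylinder door that swings on a timeline.
; Entering the Box trigger shows a W_OpenDoor prompt widget and sets CanOpen; leaving removes it, clears the flag and calls OpenDoor after a short delay.
; OpenDoor plays the timeline to lerp the Cylinder's world rotation if CanOpen is set, otherwise reverses it.
; The overlap-begin path never calls OpenDoor, and the overlaps do not filter the other actor.
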(event OnComponentBeginOverlap(Box)
  (params (OverlappedComponent :type Primitive%20Component%20Object%20Reference) (OtherActor :type Actor%20Object%20Reference) (OtherComp :type Primitive%20Component%20Object%20Reference) (OtherBodyIndex :type Integer) (bFromSweep :type Boolean) (SweepResult :type Hit%20Result%20Structure%20%28by%20ref%29))
  (bind _returnvalue (UserInterface|CreateWidget "/Game/Dima/W_OpenDoor.W_OpenDoor_C" (Game|GetPlayerController 0)))
  (UserInterface|Viewport|AddtoViewport _returnvalue 0)
  (Variables|Default|SetCanOpen true))

(event OnComponentEndOverlap(Box)
  (params (OverlappedComponent :type Primitive%20Component%20Object%20Reference) (OtherActor :type Actor%20Object%20Reference) (OtherComp :type Primitive%20Component%20Object%20Reference) (OtherBodyIndex :type Integer))
  (Widget|RemovefromParent (stale OnComponentBeginOverlap(Box) _returnvalue))
  (Variables|Default|SetCanOpen false)
  (Utilities|FlowControl|Delay 0.5)
  (CallFunction|OpenDoor))

(event Custom|OpenDoor
  (if (Variables|Default|GetCanOpen)
    (bind _value (Timeline|Time Play)
      (:Update
        (Transformation|SetWorldRotation (Variables|Default|GetCylinder) (Math|Rotator|Lerp(Rotator) "0, 0,90.000000" "35.000000,0.000000,90.000000" _value) false false)))
    (else
      (Timeline|Time Reverse))))

(fn ConstructionScript)